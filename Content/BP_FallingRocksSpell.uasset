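; BP_FallingRocksSpell is a spell actor that repeatedly drops falling rocks at random positions while it exists.
; A looping one-second timer starts on BeginPlay and is cleared when the actor is destroyed.
; Each tick of the timer spawns one to three BP_FallingRocksEffectData spells high up, passing on its owner and instigator.
; Random X/Y come from the min/max variables as absolute coordinates, not offset by the actor's location.
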(event `self.ReceiveDestroyed`
  (`KismetSystemLibrary.K2_ClearTimerHandle` (`self.TimerHandle`)))

(event `self.ReceiveBeginPlay`
  (bind _returnvalue (`KismetSystemLibrary.K2_SetTimer` self "SpawnRocksRandom" 1.0 true))
  (set `self.TimerHandle` _returnvalue))

(fn `SpawnRocksRandom`
  (bind _spawnlocationmin (`self.SpawnLocationMin`))
  (bind _spawnlocationmax (`self.SpawnLocationMax`))
  (for _ (range 1 (+ (`KismetMathLibrary.RandomIntegerInRange` 1 3) 1))
    (`SpellData.SpawnSpellOfType` "/Game/BP_FallingRocksEffectData.BP_FallingRocksEffectData_C" (`self.GetOwner`) (`self.GetInstigator`) (`KismetMathLibrary.MakeTransform` (`KismetMathLibrary.MakeVector` (`KismetMathLibrary.RandomFloatInRange` _spawnlocationmin _spawnlocationmax) (`KismetMathLibrary.RandomFloatInRange` _spawnlocationmin _spawnlocationmax) 1500.0)) (make `SpellSpawnParams` (0.0 0.0 0.0)))))

(fn `UserConstructionScript`)