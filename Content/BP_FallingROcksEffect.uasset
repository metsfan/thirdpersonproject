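; BP_FallingROcksEffect is a falling rock effect actor built around a Sphere component that varies in size and removes itself after impact.
; BeginPlay scales the Sphere independently on each axis within a random min/max range, and the construction script assigns it as the AreaShapeComponent.
; When the Sphere registers a hit, expected to be against the world, the actor sets a short lifespan so it is destroyed shortly afterward.
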(event `self.ReceiveBeginPlay`
  (bind _scalemin (`self.ScaleMin`))
  (bind _scalemax (`self.ScaleMax`))
  (`SceneComponent.SetWorldScale3D` (`self.Sphere`) (`KismetMathLibrary.MakeVector` (`KismetMathLibrary.RandomFloatInRange` _scalemin _scalemax) (`KismetMathLibrary.RandomFloatInRange` _scalemin _scalemax) (`KismetMathLibrary.RandomFloatInRange` _scalemin _scalemax))))

(event `self.Sphere.OnComponentHit`
  (params (OtherActor :type "Actor Object Reference") (OtherComp :type "PrimitiveComponent Object Reference") (NormalImpulse :type "Vector Structure") (Hit :type "HitResult Structure (by ref)"))
  ;[1 1 1] Destroy as soon as you hit (this would be the world)
  (`self.SetLifeSpan` 0.2))

(fn `UserConstructionScript`
  (set `self.AreaShapeComponent` (`self.Sphere`)))